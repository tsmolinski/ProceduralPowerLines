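; Spline-driven power line generator that places a default mesh as a spline mesh component at each spline point and strings cables between neighbors.
; The construction script places the meshes; BeginPlay places them again and adds the cables, so cables appear only at runtime.
; Cables join same-named sockets tagged "Power", with length scaled from point spacing.
; A visibility toggle refreshes each cable after setting its width.
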(event EventBeginPlay
  (bind _defaultmesh_1 (Variables|Default|GetDefaultMesh_1))
  (bind _spline (Variables|Default|GetSpline))
  (bind _spline_2 (Variables|Default|GetSpline))
  (bind _spline_3 (Variables|Default|GetSpline))
  (Utilities|Array|Clear (Variables|Default|GetPlacedMeshes_1))
  (bind _index (Utilities|FlowControl|ForLoopwithBreak 0 (- (Spline|GetNumberOfSplinePoints (Variables|Default|GetSpline)) 1))
    (:LoopBody
      (bind _returnvalue (AddComponent|AddSplineMeshComponent false (Math|Transform|MakeTransform (Spline|GetLocationatSplinePoint _spline_3 _index "Local") (Spline|GetRotationatSplinePoint _spline_3 _index "Local") "0.200000,1.000000,1.000000")))
      (Components|StaticMesh|SetStaticMesh _returnvalue _defaultmesh_1)
      (Utilities|Array|Add (Variables|Default|GetPlacedMeshes_1) _defaultmesh_1))
    (:Completed
      (for (_array_element _array_index) (Variables|Default|GetPlacedMeshes_1)
        (if (> (Utilities|Array|Length (Variables|Default|GetPlacedMeshes_1)) (+ _array_index 1))
          (for _array_element_2 (Class|StaticMesh|GetSocketsbyTag _array_element "Power")
            (bind _returnvalue_2 (AddComponent|AddCableComponent false (Math|Transform|MakeTransform (Math|Transform|TransformLocation (Math|Transform|MakeTransform (Spline|GetLocationatSplinePoint _spline _array_index "Local") (Spline|GetRotationatSplinePoint _spline _array_index "Local")) (Variables|/Script/Engine.StaticMeshSocket|GetRelativeLocation _array_element_2)) "0, 0, 0" "1.000000,1.000000,1.000000")))
            (Variables|/Script/CableComponent.CableComponent|SetEndLocation _returnvalue_2 (Math|Transform|TransformLocation (Math|Transform|MakeTransform (Spline|GetLocationatSplinePoint _spline_2 (+ _array_index 1) "Local") (Spline|GetRotationatSplinePoint _spline_2 (+ _array_index 1) "Local")) (Variables|/Script/Engine.StaticMeshSocket|GetRelativeLocation (Class|StaticMesh|FindSocket (Utilities|Array|Get(acopy) (Variables|Default|GetPlacedMeshes_1) (+ _array_index 1)) (Variables|/Script/Engine.StaticMeshSocket|GetSocketName _array_element_2)))))
            (Variables|/Script/CableComponent.CableComponent|SetCableLength _returnvalue_2 (* (Variables|Default|GetCablesLenghtMultiplier_1) (Math|Vector|VectorLength (- (Spline|GetLocationatSplinePoint _spline _array_index "Local") (Spline|GetLocationatSplinePoint _spline_2 (+ _array_index 1) "Local")))))
            (Variables|/Script/CableComponent.CableComponent|SetCableWidth _returnvalue_2 (Variables|Default|GetCablesWidth_1))
            ;[1 1 1] It's needed to "rerender" cables after changing it's width.
            (Rendering|SetVisibility _returnvalue_2 false false)
            (Rendering|SetVisibility _returnvalue_2 true false)))))))

(fn ConstructionScript
  (bind _spline (Variables|Default|GetSpline))
  (bind _defaultmesh_1 (Variables|Default|GetDefaultMesh_1))
  (Utilities|Array|Clear (Variables|Default|GetPlacedMeshes_1))
  (bind _index (Utilities|FlowControl|ForLoopwithBreak 0 (- (Spline|GetNumberOfSplinePoints (Variables|Default|GetSpline)) 1))
    (:LoopBody
      (bind _returnvalue (AddComponent|AddSplineMeshComponent false (Math|Transform|MakeTransform (Spline|GetLocationatSplinePoint _spline _index "Local") (Spline|GetRotationatSplinePoint _spline _index "Local") "0.200000,1.000000,1.000000")))
      (Components|StaticMesh|SetStaticMesh _returnvalue _defaultmesh_1)
      (Utilities|Array|Add (Variables|Default|GetPlacedMeshes_1) _defaultmesh_1))))